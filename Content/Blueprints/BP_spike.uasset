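; BP_spike is a spike hazard whose Cone component destroys any actor that triggers its hit event.
; An Interaction event records the Cone's current relative height and plays a Timeline that offsets it along Z by the track value scaled by a Move variable.
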(event `self.Cone.OnComponentHit`
  (params (HitComponent :type "PrimitiveComponent Object Reference") (OtherActor :type "Actor Object Reference") (OtherComp :type "PrimitiveComponent Object Reference") (NormalImpulse :type "Vector Structure") (Hit :type "HitResult Structure (by ref)"))
  (`self.K2_DestroyActor` OtherActor))

(event `/Game/Blueprints/BPI_Interact.Interaction`
  (bind _cone (`self.Cone`))
  (bind (_relativelocation_x _relativelocation_y) (`KismetMathLibrary.BreakVector` (`SceneComponent.RelativeLocation` _cone)))
  (bind (_relativelocation_x_2 _relativelocation_y_2 _relativelocation_z) (`KismetMathLibrary.BreakVector` (`SceneComponent.RelativeLocation` (`self.Cone`))))
  (set `self.start` _relativelocation_z)
  (bind (_direction _newtrack_0) (`Timeline|Timeline`)
    (:`Update`
      (`SceneComponent.K2_SetRelativeLocation` _cone (`KismetMathLibrary.MakeVector` _relativelocation_x _relativelocation_y (+ (* _newtrack_0 (`self.move`)) (`self.start`))) false false))))

(fn `UserConstructionScript`)