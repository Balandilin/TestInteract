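; BP_hammer is an interactive hammer actor that swings when triggered and destroys what its Cube component hits.
; The Interaction event stores the Cylinder's relative roll, then plays a timeline that adds its track value times Rotationage to that roll, leaving pitch and yaw unchanged.
; Cube's hit event destroys the other actor without any filtering, whether or not a swing is playing.
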(event `self.Cube.OnComponentHit`
  (params (HitComponent :type "PrimitiveComponent Object Reference") (OtherActor :type "Actor Object Reference") (OtherComp :type "PrimitiveComponent Object Reference") (NormalImpulse :type "Vector Structure") (Hit :type "HitResult Structure (by ref)"))
  (`self.K2_DestroyActor` OtherActor))

(event `/Game/Blueprints/BPI_Interact.Interaction`
  (bind _cylinder (`self.Cylinder`))
  (bind (_relativerotation_roll _relativerotation_pitch _relativerotation_yaw) (`KismetMathLibrary.BreakRotator` (`SceneComponent.RelativeRotation` _cylinder)))
  (bind _relativerotation_roll_2 (`KismetMathLibrary.BreakRotator` (`SceneComponent.RelativeRotation` (`self.Cylinder`))))
  (set `self.start` _relativerotation_roll_2)
  (bind (_direction _newtrack_0) (`Timeline|Timeline`)
    (:`Update`
      (`SceneComponent.K2_SetRelativeRotation` _cylinder (`KismetMathLibrary.MakeRotator` (+ (`self.start`) (* _newtrack_0 (`self.rotationage`))) _relativerotation_pitch _relativerotation_yaw) false false))))

(fn `UserConstructionScript`)