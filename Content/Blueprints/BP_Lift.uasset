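; Lift actor that moves its Cube component vertically when an interaction fires.
; On BeginPlay it casts the player character to BP_Player and binds its interaction event to the LaunchAllInteraction dispatcher.
; Interaction stores the cube's current relative Z, then a timeline offsets it from that height by its track value scaled by MovementZ.
; A separate AllCall event only prints a debug greeting.
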(event `self.ReceiveBeginPlay`
  (bind _asbp_player (cast `/Game/Blueprints/BP_Player` (`GameplayStatics.GetPlayerCharacter` 0)))
  (add `/Game/Blueprints/BP_Player.LaunchAllInteraction` _asbp_player (delegate `/Game/Blueprints/BPI_Interact.Interaction`)))

(event `AllCall`
  (`KismetSystemLibrary.PrintString` "Hello"))

(event `/Game/Blueprints/BPI_Interact.Interaction`
  (bind _cube (`self.Cube`))
  (bind (_relativelocation_x _relativelocation_y _relativelocation_z) (`KismetMathLibrary.BreakVector` (`SceneComponent.RelativeLocation` (`self.Cube`))))
  (bind (_relativelocation_x_2 _relativelocation_y_2) (`KismetMathLibrary.BreakVector` (`SceneComponent.RelativeLocation` _cube)))
  (set `self.StartingPoint` _relativelocation_z)
  (bind (_direction _newtrack_0) (`Timeline|Timeline`)
    (:`Update`
      (`SceneComponent.K2_SetRelativeLocation` _cube (`KismetMathLibrary.MakeVector` _relativelocation_x_2 _relativelocation_y_2 (+ (`self.StartingPoint`) (* _newtrack_0 (`self.MovementZ`)))) false false))))

(fn `UserConstructionScript`)