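; BP_ChangeColor is an interactable actor whose cube cycles through colors when the player triggers an interaction.
; On BeginPlay it casts the player character to BP_Player and binds to its LaunchAllInteraction event dispatcher.
; Each interaction advances a wrapping index over three entries of a Color array and writes that color to the cube's material "Color" vector parameter.
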(event `self.ReceiveBeginPlay`
  (bind _asbp_player (cast `/Game/Blueprints/BP_Player` (`GameplayStatics.GetPlayerCharacter` 0)))
  (add `/Game/Blueprints/BP_Player.LaunchAllInteraction` _asbp_player (delegate `/Game/Blueprints/BPI_Interact.Interaction`)))

(event `/Game/Blueprints/BPI_Interact.Interaction`
  (`self.change color`))

(fn `change color`
  (`/Engine/EditorBlueprintResources/StandardMacros.IncrementInt` (`self.Array Index`)
    (:`  `
      (if (>= (`self.Array Index`) 3)
        (set `self.Array Index` 0))
      (`MeshComponent.SetVectorParameterValueOnMaterials` (`self.Cube`) "Color" (`|GetArrayItem` (`self.color`) (`self.Array Index`))))))

(fn `UserConstructionScript`)